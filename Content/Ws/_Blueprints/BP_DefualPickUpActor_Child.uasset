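; Child pickup actor Blueprint, apparently a test or template variant of the default pickup, with three use stages: once, last and end.
; CE_UseOnce, CE_UseLast and CE_UseEnd only print their stage name as debug text.
; A parallel set of events without underscores each makes a same-named call.
; BeginPlay, overlap and Tick are disabled stubs, and construction defers to the parent.
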(event `CE_UseOnce`
  (`KismetSystemLibrary.PrintString` "UseOnce"))

(event `/Game/Ws/_Blueprints/Interface/INF_PickUp.CE_Use_Once`
  (`self.CE_UseOnce`))

(event `/Game/Ws/_Blueprints/Interface/INF_PickUp.CE_Use_Last`
  (`self.CE_UseLast`))

(event `CE_UseLast`
  (`KismetSystemLibrary.PrintString` "UseLast"))

(event `/Game/Ws/_Blueprints/Interface/INF_PickUp.CE_Use_End`
  (`self.CE_UseEnd`))

(event `CE_UseEnd`
  (`KismetSystemLibrary.PrintString` "UseEnd"))

(fn `UserConstructionScript`
  (`parent.UserConstructionScript`))