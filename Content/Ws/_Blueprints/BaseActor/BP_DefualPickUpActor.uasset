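; Base pickup actor that can act as a trigger volume when IsTrigger is set.
; In that mode the construction script adds a collision-free static mesh with the configured material, snaps it to TriggerBox and scales the box.
; The server trigger event relays through a multicast event to the trigger event dispatcher and prints a debug message.
; BeginPlay registers the actor as parent of its ACDebug component, and the AdsEvent hook is empty.
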(event `self.ReceiveBeginPlay`
  (set `/Game/Ws/_Blueprints/ActorComponent/AC_Debug.Parent` self (`self.AC_Debug`)))

(event `CE_TriggerEvent_Server`
  (if (`self.bIsTrigger`)
    (`self.CE_TriggerEvent_Multicast`)))

(event `CE_TriggerEvent_Multicast`
  (`self.ED_TriggerEvent`)
  (`KismetSystemLibrary.PrintString` "作为触发器事件"))

(event `CE_AdsEvent`)

(fn `UserConstructionScript`
  (if (`self.bIsTrigger`)
    (bind _returnvalue (`AddComponent|NODE_AddStaticMeshComponent-0`))
    (bind _output_get (set `self.StaticMesh` _returnvalue))
    (`SceneComponent.K2_AttachToComponent` _output_get (`self.TriggerBox`) "None" "SnapToTarget" "SnapToTarget" "SnapToTarget" true)
    (`StaticMeshComponent.SetStaticMesh` _output_get (`self.TriggerMesh`))
    (`PrimitiveComponent.SetCollisionEnabled` _returnvalue "NoCollision")
    (`PrimitiveComponent.SetMaterial` _returnvalue 0 (`self.Material`))
    (`SceneComponent.SetRelativeScale3D` (`self.TriggerBox`) (`self.Scale`))))