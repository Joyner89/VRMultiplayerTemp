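; BP_Adsorption is a snap-point actor that pickup actors can attach to, showing a preview mesh while a matching one overlaps its box.
; On the server, overlap begin and end set or clear the pickup's AdsorptionActor and toggle replicated ShowMesh, whose OnRep updates mesh visibility.
; The server adsorption event multicasts the adsorption dispatcher and hides the preview; leaving the box fires a no-adsorption dispatcher on the server.
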(event `self.ReceiveBeginPlay`
  (`SceneComponent.SetVisibility` (`self.StaticMesh`) false false))

(event `self.Box.OnComponentBeginOverlap`
  (params (OverlappedComponent :type "PrimitiveComponent Object Reference") (OtherActor :type "Actor Object Reference") (OtherComp :type "PrimitiveComponent Object Reference") (OtherBodyIndex :type Integer) (bFromSweep :type Boolean) (SweepResult :type "HitResult Structure (by ref)"))
  (if (`KismetSystemLibrary.IsServer`)
    (if (== (`GameplayStatics.GetObjectClass` OtherActor) (`self.RelevanceActorClass`))
      (bind _asbp_defual_pick_up_actor (cast `/Game/Ws/_Blueprints/BaseActor/BP_DefualPickUpActor` OtherActor))
      (set `/Game/Ws/_Blueprints/BaseActor/BP_DefualPickUpActor.AdsorptionActor` self _asbp_defual_pick_up_actor)
      (set `self.bShowMesh` true))))

(event `self.Box.OnComponentEndOverlap`
  (params (OverlappedComponent :type "PrimitiveComponent Object Reference") (OtherActor :type "Actor Object Reference") (OtherComp :type "PrimitiveComponent Object Reference") (OtherBodyIndex :type Integer))
  (if (`KismetSystemLibrary.IsServer`)
    (if (== (`GameplayStatics.GetObjectClass` OtherActor) (`self.RelevanceActorClass`))
      (bind _asbp_defual_pick_up_actor (cast `/Game/Ws/_Blueprints/BaseActor/BP_DefualPickUpActor` OtherActor))
      (set `/Game/Ws/_Blueprints/BaseActor/BP_DefualPickUpActor.AdsorptionActor` null _asbp_defual_pick_up_actor)
      (set `self.bShowMesh` false)
      (`self.ED_NoAdsorptionEvent`))))

(event `CE_AdsorptionEvent_Server`
  (`self.CE_AdsorptionEvent_Multicast`)
  (`KismetSystemLibrary.PrintString` "吸附事件")
  (set `self.bShowMesh` false))

(event `CE_AdsorptionEvent_Multicast`
  (`self.ED_AdsorptionEvent` self))

(fn `OnRep_bShowMesh`
  (`SceneComponent.SetVisibility` (`self.StaticMesh`) (`self.bShowMesh`) false))

(fn `UserConstructionScript`)