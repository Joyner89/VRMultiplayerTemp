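; PC_MainController is the main player controller, setting up either the menu map or gameplay maps on BeginPlay.
; On _MianMap it only creates the WBP_Mian widget.
; Elsewhere it shows the cursor and adds the Enhanced Input context.
; If locally controlled, it looks up the GameInstance's platform and ID in DT_PlatformPawn, then asks GM_MainGameMode to spawn that pawn.
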(event `self.ReceiveBeginPlay`
  (bind (_returnvalue _platform _id) (`/Game/Ws/_Blueprints/FunctionLibraty/FL_ProjectFunction.F_GetPlatformPawnID_FromGameInstance`))
  (bind _returnvalue_2 (subsystem `EnhancedInputLocalPlayerSubsystem`))
  (bind _returnvalue_3 (`GameplayStatics.GetCurrentLevelName` true))
  (if (`KismetStringLibrary.EqualEqual_StrStr` _returnvalue_3 "_MianMap")
    (`self.CE_CreateWidget` "/Game/Ws/_Blueprints/UI_BP/Widget/WBP_Mian.WBP_Mian_C" self) ; 只在主关卡加载UI
    (else
      (`|ExecutionSequence`
        (:`then_0`
          (set `self.bShowMouseCursor` true)
          (`/Engine/EditorBlueprintResources/StandardMacros.IsValid` _returnvalue_2
            (:`Is Valid`
              (`EnhancedInputSubsystemInterface.AddMappingContext` _returnvalue_2 "/Game/Ws/_Blueprints/Input/IMC_TestDefault.IMC_TestDefault" 0 (struct)))))
        (:`then_1`
          (if (and (`self.IsLocalController`) _returnvalue)
            (bind _returnvalue_4 (`|GetDataTableRow` "/Game/Ws/_Blueprints/DataTable/DT_PlatformPawn.DT_PlatformPawn" (`KismetStringLibrary.Conv_StringToName` (`KismetStringLibrary.Concat_StrStr` (`|GetEnumeratorNameAsString` _platform) "-" (`KismetStringLibrary.Conv_IntToString` _id))))
              (:`then`
                (bind (_platform_2 _id_2 _pawn) (break `/Game/Ws/_Blueprints/Data/ST_PlatformPawn` _returnvalue_4))
                (`self.CE_SpawnPawnFromGameMode` _pawn _platform_2 _id_2)))))))))

(event `CE_CreateWidget`
  (params (Class :type "UserWidget Class Reference") (OwningPlayer :type "PlayerController Object Reference"))
  ;[0 0 0] 创建UI并添加到屏幕
  (bind _returnvalue (`|CreateWidget` Class OwningPlayer))
  (`UserWidget.AddToViewport` _returnvalue 0))

(event `CE_SpawnPawnFromGameMode`
  (params (Pawn :type "Pawn Class Reference") (Platform :type "/Game/Ws/_Blueprints/Data/Enum/Enum_Platform Enum" :default "NewEnumerator0") (ID :type Integer))
  ;[0 0 0] 调用GameMode中的创建Pawn的方法
  (bind _asgm_main_game_mode (cast `/Game/Ws/_Blueprints/GameMode/GM_MainGameMode` (`GameplayStatics.GetGameMode`)))
  (`/Game/Ws/_Blueprints/GameMode/GM_MainGameMode.CE_SpawnPawn` _asgm_main_game_mode self Pawn Platform ID))

(fn `UserConstructionScript`)